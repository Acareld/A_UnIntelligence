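; BP_InspectorGameMode is a game mode that manages the level's UI from start to finish.
; On BeginPlay it creates a Timer widget, stores it as InGameUI and adds it to the viewport.
; OnLevelEnded shows WBP_EndScreen, removes the timer widget, switches to UI-only input with a visible cursor and pauses the game.
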(event EventBeginPlay
  (bind _returnvalue (UserInterface|CreateWidget "/Game/UI/Timer.Timer_C"))
  (bind _output_get (Variables|Default|SetInGameUI _returnvalue))
  (UserInterface|Viewport|AddtoViewport _output_get 0))

(event EventTick
  (params (DeltaSeconds :type Float%20%28single-precision%29)))

(event EventOnLevelEnded
  (bind _returnvalue (Game|GetPlayerController 0))
  (bind _returnvalue_2 (UserInterface|CreateWidget "/Game/UI/EndScreen/WBP_EndScreen.WBP_EndScreen_C" _returnvalue))
  (UserInterface|Viewport|AddtoViewport _returnvalue_2 0)
  (Widget|RemovefromParent (Variables|Default|GetInGameUI))
  (Input|SetInputModeUIOnly _returnvalue 0 "DoNotLock" false)
  (Variables|/Script/Engine.PlayerController|SetbShowMouseCursor _returnvalue true)
  (Game|SetGamePaused true))

(fn ConstructionScript)